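; BP_Player_Old is a player Blueprint that stands upright on a spherical planet and is pulled toward its center.
; On BeginPlay it gets the planet from BP_LocalDatabaseActor and disables mesh collision.
; Each Tick it rotates its up axis away from the planet, keeping its forward vector projected on the tangent plane.
; A trace toward the planet gates the gravity force on the capsule, applied only beyond DistanceToGround.
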(event EventBeginPlay
  (bind _outactors (Actor|GetAllActorsOfClass "/Game/Blueprints/BP_LocalDatabaseActor.BP_LocalDatabaseActor_C"))
  (Variables|Default|SetPlanet (Variables|/Game/Blueprints/BP_LocalDatabaseActor.BP_LocalDatabaseActor_C|GetPlanet (Utilities|Array|Get(acopy) _outactors)))
  (Collision|SetCollisionEnabled (Variables|Character|GetMesh) "NoCollision"))

(event Collision|EventActorBeginOverlap
  (params (OtherActor :type Actor%20Object%20Reference)))

(event EventTick
  (params (DeltaSeconds :type Float%20%28single-precision%29))
  (bind _returnvalue (Transformation|GetActorRotation))
  (bind _returnvalue_2 (Transformation|GetActorLocation))
  (bind _planet (Variables|Default|GetPlanet))
  (bind _planet_2 (Variables|Default|GetPlanet))
  (bind _returnvalue_3 (Transformation|GetActorLocation _planet))
  (bind _returnvalue_4 (Math|Vector|GetForwardVector _returnvalue))
  (bind _returnvalue_5 (- _returnvalue_3 _returnvalue_2))
  (bind _returnvalue_6 (Math|Vector|Normalize _returnvalue_5))
  (Utilities|IsValid _planet_2
    (:Is%20Valid
      (Transformation|SetActorRotation (Math|Rotator|MakeRotfromXZ (- _returnvalue_4 (Math|Vector|ProjectVectorontoVector _returnvalue_4 _returnvalue_6)) (Math|Vector|NegateVector _returnvalue_6)))
      (bind _outhit (Collision|LineTraceByChannel (Transformation|GetActorLocation) (Transformation|GetActorLocation _planet_2) "TraceTypeQuery3" false 0 "None" true "(R=1.000000,G=0.000000,B=0.000000,A=1.000000)" "(R=0.000000,G=1.000000,B=0.000000,A=1.000000)" DeltaSeconds))
      (if (not (<= (.Distance (Collision|BreakHitResult _outhit)) (Variables|Default|GetDistanceToGround)))
        (Physics|AddForce (Variables|Collision|GetCapsuleComponent) (* _returnvalue_6 (Variables|Default|GetGravityMultiplier)) "None" false)))))

(fn ConstructionScript)