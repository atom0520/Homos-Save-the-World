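; AI controller for a planet-dwelling human in an LD42 game that grows up, wanders, then seeks a mate to breed.
; Tick counts down maturity, then runs an Idle/Wander/Chase state machine moving the capsule with forces.
; A sphere overlap picks the nearest unpaired, mature, opposite-gender human and links both controllers as targets.
; Within mating range, both parents are disabled and children spawn around their midpoint, alternating gender, via the game mode.
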(event EventBeginPlay)

(event EventTick
  (params (DeltaSeconds :type Float%20%28single-precision%29))
  (bind _returnvalue (Pawn|GetControlledPawn))
  (bind _target (Variables|Default|GetTarget))
  (bind _target_2 (Variables|Default|GetTarget))
  (bind _returnvalue_2 (Transformation|GetActorLocation _target))
  (Utilities|IsValid (Variables|Default|GetControlledHumanBP)
    (:Is%20Valid
      (Utilities|FlowControl|Sequence
        (:then_0
          (if (Variables|/Game/Blueprints/BP_Human_Old.BP_Human_Old_C|GetMature (Variables|Default|GetControlledHumanBP))
            (if (Variables|Default|GetFoundTarget)
              (bind _asbp_ld42game_mode_old (Utilities|Casting|CastToBP_LD42GameMode_Old (Game|GetGameMode)))
              (if (not (Variables|/Game/Blueprints/BP_LD42GameMode_Old.BP_LD42GameMode_Old_C|GetIsGameOver _asbp_ld42game_mode_old))
                (Variables|Default|SetAIState "NewEnumerator2"))
              (else
                (bind _returnvalue_3 (CallFunction|SearchforTarget))
                (if _returnvalue_3
                  (Variables|Default|SetAIState "NewEnumerator2"))))
            (elif (<= (Variables|Default|GetGrowthTimer) 0.0)
              (Default|GrowUp (Variables|Default|GetControlledHumanBP))
              (else
                (Variables|Default|SetGrowthTimer (- (Variables|Default|GetGrowthTimer) DeltaSeconds))))))
        (:then_1
          (switch Utilities|FlowControl|Switch|SwitchonEHumanAIState (Variables|Default|GetAIState)
            (:NewEnumerator0
              (Utilities|FlowControl|Delay (Math|Random|RandomFloatinRange 2.0 3.0))
              (Variables|Default|SetAIState "NewEnumerator1")
              (goto _label Reset))
            (:NewEnumerator1
              (Utilities|FlowControl|Sequence
                (:then_0
                  (Utilities|FlowControl|DoOnce false :!label _label
                    (:Completed
                      (Transformation|AddActorLocalRotation (Variables|Default|GetControlledHumanBP) (Math|Rotator|MakeRotator 0.0 0.0 (Math|Random|RandomFloatinRange -1.8e+02 1.8e+02)) false false)
                      (Variables|Default|SetAITimer (Math|Random|RandomFloatinRange 2.0 3.0)))))
                (:then_1
                  (if (<= (Variables|Default|GetAITimer) 0.0)
                    (Variables|Default|SetAIState "NewEnumerator0")
                    (else
                      (Variables|Default|SetAITimer (- (Variables|Default|GetAITimer) DeltaSeconds))
                      (Utilities|IsValid (Variables|Default|GetControlledHumanBP)
                        (:Is%20Valid
                          (Physics|AddForce (Variables|/Game/Blueprints/BP_Human_Old.BP_Human_Old_C|GetCapsuleComponent (Variables|Default|GetControlledHumanBP)) (* (Math|Vector|GetForwardVector (Transformation|GetActorRotation (Variables|Default|GetControlledHumanBP))) (Variables|Default|GetMoveInputMultiplier)) "None" false))))))))
            (:NewEnumerator2
              (bind _asbp_ld42game_mode_old_2 (Utilities|Casting|CastToBP_LD42GameMode_Old (Game|GetGameMode)))
              (if (Variables|/Game/Blueprints/BP_LD42GameMode_Old.BP_LD42GameMode_Old_C|GetIsGameOver _asbp_ld42game_mode_old_2)
                (Variables|Default|SetAIState "NewEnumerator0" :!label _label_2)
                (elif (Variables|Default|GetFoundTarget)
                  (if (== (Variables|/Game/Blueprints/BP_Human_Old.BP_Human_Old_C|GetGender _target_2) (Variables|/Game/Blueprints/BP_Human_Old.BP_Human_Old_C|GetGender (Variables|Default|GetControlledHumanBP)))
                    (Variables|Default|SetFoundTarget false)
                    (goto _label_2)
                    (else
                      (Transformation|SetActorRotation (Variables|Default|GetControlledHumanBP) (Math|Rotator|MakeRotfromZX (Math|Vector|GetUpVector (Transformation|GetActorRotation (Variables|Default|GetControlledHumanBP))) (- (- (Transformation|GetActorLocation _target_2) (Transformation|GetActorLocation (Variables|Default|GetControlledHumanBP))) (Math|Vector|ProjectVectorontoVector (- (Transformation|GetActorLocation _target_2) (Transformation|GetActorLocation (Variables|Default|GetControlledHumanBP))) (Math|Vector|NegateVector (Math|Vector|GetUpVector (Transformation|GetActorRotation (Variables|Default|GetControlledHumanBP))))))))
                      (if (<= (Math|Vector|VectorLength (- (Transformation|GetActorLocation _target_2) (Transformation|GetActorLocation (Variables|Default|GetControlledHumanBP)))) (Variables|Default|GetMateDistance))
                        (Effects|SpawnEmitteratLocation "/Game/Paticles/PS_Love.PS_Love" (* (+ _returnvalue_2 (Transformation|GetActorLocation (Variables|Default|GetControlledHumanBP))) 0.5) "0, 0, 0" "1.000000,1.000000,1.000000" true "AutoRelease")
                        (Default|SetEnabled _target false)
                        (Default|SetEnabled (Variables|Default|GetControlledHumanBP) false)
                        (bind _asbp_ld42game_mode_old_3 (Utilities|Casting|CastToBP_LD42GameMode_Old (Game|GetGameMode)))
                        (Default|UpdateNumberOfHumans _asbp_ld42game_mode_old_3 (Variables|/Game/Blueprints/BP_Human_Old.BP_Human_Old_C|GetGender _target) -1)
                        (Default|UpdateNumberOfHumans _asbp_ld42game_mode_old_3 (Variables|/Game/Blueprints/BP_Human_Old.BP_Human_Old_C|GetGender (Variables|Default|GetControlledHumanBP)) -1)
                        (for _index (range 0 (Math|Random|RandomIntegerinRange (Variables|Default|GetMinBearChildrenNumber) (Variables|Default|GetMaxBearChildrenNumber)))
                          (Utilities|FlowControl|FlipFlop
                            (:A
                              (Default|SpawnHuman _asbp_ld42game_mode_old_3 (+ (* (+ _returnvalue_2 (Transformation|GetActorLocation (Variables|Default|GetControlledHumanBP))) 0.5) (* (Math|Vector|RotateVectorAroundAxis (Math|Vector|Normalize (- _returnvalue_2 (Transformation|GetActorLocation (Variables|Default|GetControlledHumanBP)))) (Math|Random|RandomFloatinRange 0.0 1.8e+02) (- (Transformation|GetActorLocation (Variables|/Game/Blueprints/BP_Human_Old.BP_Human_Old_C|GetPlanet (Variables|Default|GetControlledHumanBP))) (* (+ _returnvalue_2 (Transformation|GetActorLocation (Variables|Default|GetControlledHumanBP))) 0.5))) 64.0)) (Transformation|GetActorRotation _target) 0 false))
                            (:B
                              (Default|SpawnHuman _asbp_ld42game_mode_old_3 (+ (* (+ _returnvalue_2 (Transformation|GetActorLocation (Variables|Default|GetControlledHumanBP))) 0.5) (* (Math|Vector|RotateVectorAroundAxis (Math|Vector|Normalize (- _returnvalue_2 (Transformation|GetActorLocation (Variables|Default|GetControlledHumanBP)))) (Math|Random|RandomFloatinRange -1.8e+02 0.0) (- (Transformation|GetActorLocation (Variables|/Game/Blueprints/BP_Human_Old.BP_Human_Old_C|GetPlanet (Variables|Default|GetControlledHumanBP))) (* (+ _returnvalue_2 (Transformation|GetActorLocation (Variables|Default|GetControlledHumanBP))) 0.5))) 64.0)) (Transformation|GetActorRotation (Variables|Default|GetControlledHumanBP)) 1 false))))
                        (else
                          (Physics|AddForce (Variables|/Game/Blueprints/BP_Human_Old.BP_Human_Old_C|GetCapsuleComponent (Variables|Default|GetControlledHumanBP)) (* (Math|Vector|GetForwardVector (Transformation|GetActorRotation (Variables|Default|GetControlledHumanBP))) (Variables|Default|GetMoveInputMultiplier)) "None" false)))))
                  (else
                    (goto _label_2)))))))))
    (:Is%20Not%20Valid
      (Utilities|IsValid _returnvalue
        (:Is%20Valid
          (bind _asbp_human_old (Utilities|Casting|CastToBP_Human_Old _returnvalue))
          (Variables|Default|SetControlledHumanBP _asbp_human_old))))))

(fn ConstructionScript)

(fn SearchforTarget
  (bind _controlledhumanbp (Variables|Default|GetControlledHumanBP))
  (bind _returnvalue (Transformation|GetActorLocation _controlledhumanbp))
  (bind (_outactors _returnvalue_2) (Collision|SphereOverlapActors _returnvalue (Variables|Default|GetTargetSearchRange) (Utilities|Array|MakeArray "ObjectTypeQuery3") "/Game/Blueprints/BP_Human_Old.BP_Human_Old_C" (Utilities|Array|MakeArray (Variables|Default|GetControlledHumanBP) (Game|Player|GetPlayerPawn 0))))
  (if _returnvalue_2
    (Variables|Default|SetClosestTargetDistance (+ (Variables|Default|GetTargetSearchRange) 1e+02))
    (for _array_element _outactors
      (bind _asbp_human_old (Utilities|Casting|CastToBP_Human_Old _array_element))
      (if (Variables|/Game/Blueprints/BP_Human_Old.BP_Human_Old_C|GetMature _asbp_human_old)
        (bind _ashuman_aicontroller_bp_old (Utilities|Casting|CastToBP_HumanAIController_Old (Pawn|GetController _asbp_human_old)))
        (if (not (Variables|BP_HumanAIController_Old_C|GetFoundTarget _ashuman_aicontroller_bp_old))
          (if (not (== (Variables|/Game/Blueprints/BP_Human_Old.BP_Human_Old_C|GetGender (Variables|Default|GetControlledHumanBP)) (Variables|/Game/Blueprints/BP_Human_Old.BP_Human_Old_C|GetGender _asbp_human_old)))
            (if (not (<= (Variables|Default|GetClosestTargetDistance) (Math|Vector|VectorLength (- _returnvalue (Transformation|GetActorLocation _array_element)))))
              (Variables|Default|SetTarget _asbp_human_old)
              (Variables|Default|SetFoundTarget true)
              (Variables|Default|SetClosestTargetDistance (Math|Vector|VectorLength (- _returnvalue (Transformation|GetActorLocation _array_element)))))))))
    (if (Variables|Default|GetFoundTarget)
      (bind _ashuman_aicontroller_bp_old_2 (Utilities|Casting|CastToBP_HumanAIController_Old (Pawn|GetController (Variables|Default|GetTarget))))
      (Variables|BP_HumanAIController_Old_C|SetTarget _ashuman_aicontroller_bp_old_2 (Variables|Default|GetControlledHumanBP))
      (Variables|BP_HumanAIController_Old_C|SetFoundTarget _ashuman_aicontroller_bp_old_2 true)
      (return true)
      (else
        (return false)))
    (else
      (return false))))

(fn Initialize
  (Variables|Default|SetGrowthTimer (Variables|Default|GetTimeToMature))
  (Variables|Default|SetAIState "NewEnumerator0")
  (Variables|Default|SetFoundTarget false))