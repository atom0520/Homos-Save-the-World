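; Player controller that drives BP_Player, lets the player change the gender of the aimed human, and toggles pause.
; Movement axes push the player's capsule with forces along the pawn's forward and right vectors.
; Turn rotates the pawn, while the look axis pitches its camera.
; Fire calls ChangeGender on a valid AimedHuman, which is not set here, and plays a sound there; P flip-flops game pause.
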(event EventBeginPlay)

(event EventTick
  (params (DeltaSeconds :type Float%20%28single-precision%29)))

(event Input|ActionEvents|InputActionFire
  (params (Key :type Key%20Structure))
  (bind _aimedhuman (Variables|Default|GetAimedHuman))
  (:Pressed
    (Utilities|IsValid _aimedhuman
      (:Is%20Valid
        (Class|Human|ChangeGender _aimedhuman)
        (Audio|PlaySoundatLocation "/Game/Sounds/S_ChangeGender.S_ChangeGender" (Transformation|GetActorLocation _aimedhuman) "0, 0, 0" 1.0 1.0 0.0 0 0 0)))))

(event Input|AxisEvents|InputAxisTurn
  (params (AxisValue :type Float%20%28single-precision%29))
  (Transformation|AddActorLocalRotation (Pawn|GetControlledPawn) (Math|Rotator|MakeRotator 0.0 0.0 (* AxisValue (Variables|Default|GetTurnInputMultiplier))) false false))

(event Input|AxisEvents|InputAxisLoopUp
  (params (AxisValue :type Float%20%28single-precision%29))
  (bind _asbp_player (Utilities|Casting|CastToBP_Player (Pawn|GetControlledPawn)))
  (Transformation|AddLocalRotation (Variables|/Game/Blueprints/BP_Player.BP_Player_C|GetCamera _asbp_player) (Math|Rotator|MakeRotator 0.0 (* AxisValue (Variables|Default|GetTurnInputMultiplier)) 0.0) false false))

(event Input|AxisEvents|InputAxisMoveForward
  (params (AxisValue :type Float%20%28single-precision%29))
  (bind _returnvalue (Pawn|GetControlledPawn))
  (bind _asbp_player (Utilities|Casting|CastToBP_Player _returnvalue))
  (Physics|AddForce (Variables|/Script/LD42.MyPawn|GetCapsuleComponent _asbp_player) (* (Math|Vector|GetForwardVector (Transformation|GetActorRotation _returnvalue)) (* AxisValue (Variables|Default|GetMoveInputMultiplier))) "None" false))

(event Input|AxisEvents|InputAxisMoveRight
  (params (AxisValue :type Float%20%28single-precision%29))
  (bind _returnvalue (Pawn|GetControlledPawn))
  (bind _asbp_player (Utilities|Casting|CastToBP_Player _returnvalue))
  (Physics|AddForce (Variables|/Script/LD42.MyPawn|GetCapsuleComponent _asbp_player) (* (Math|Vector|GetRightVector (Transformation|GetActorRotation _returnvalue)) (* AxisValue (Variables|Default|GetMoveInputMultiplier))) "None" false))

(event Input|KeyboardEvents|P
  (params (Key :type Key%20Structure))
  (:Pressed
    (bind _isa (Utilities|FlowControl|FlipFlop)
      (:A
        _)
      (:B
        _))
    (Game|SetGamePaused _isa)))

(fn ConstructionScript)