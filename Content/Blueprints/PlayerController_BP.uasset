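; Player controller for the LD42 game that lets the player move, look, aim at humans and switch their gender.
; Movement input pushes the character's capsule with forces, while look input rotates the pawn for yaw and its camera for pitch.
; Until game over, Tick line-traces through the crosshair to set the aimed human and show its gender icon on the HUD.
; Fire changes that human's gender with a sound; Quit exits.
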(event EventBeginPlay
  (bind _asld42game_mode_bp (Utilities|Casting|CastToLD42GameMode_BP (Game|GetGameMode)))
  (Variables|Default|SetCrosshairGenderImage (Variables|/Game/Blueprints/GUIWidget_BP.GUIWidget_BP_C|GetGenderImage (Variables|/Game/Blueprints/LD42GameMode_BP.LD42GameMode_BP_C|GetGUIWidget _asld42game_mode_bp))))

(event EventTick
  (params (DeltaSeconds :type Float%20%28single-precision%29))
  (bind (_sizex _sizey) (HUD|GetViewportSize))
  (bind _self self)
  (bind _crosshairlocationx (Variables|Default|GetCrosshairLocationX))
  (bind _crosshairgenderimage (Variables|Default|GetCrosshairGenderImage))
  (bind _crosshairgenderimage_2 (Variables|Default|GetCrosshairGenderImage))
  (bind _crosshairlocationy (Variables|Default|GetCrosshairLocationY))
  (bind _returnvalue (* _sizex _crosshairlocationx))
  (bind _returnvalue_2 (* _sizey _crosshairlocationy))
  (bind _returnvalue_3 (Math|Vector2D|MakeVector2D _returnvalue _returnvalue_2))
  (bind (_worldposition _worlddirection) (Class|GameplayStatics|DeprojectScreentoWorld _self _returnvalue_3))
  (bind _asld42game_mode_bp (Utilities|Casting|CastToLD42GameMode_BP (Game|GetGameMode)))
  (if (Variables|/Game/Blueprints/LD42GameMode_BP.LD42GameMode_BP_C|GetIsGameOver _asld42game_mode_bp)
    (Variables|Default|SetAimedHuman 0 :!label _label)
    (Utilities|IsValid _crosshairgenderimage
      (:Is%20Valid
        (Widget|SetVisibility _crosshairgenderimage "Hidden")))
    (else
      (bind (_outhit _returnvalue_4) (Collision|LineTraceByChannel _worldposition (+ _worldposition (* _worlddirection (Variables|Default|GetCrosshairLineTraceRange))) "TraceTypeQuery4" false 0 "None"))
      (if _returnvalue_4
        (bind _ashuman_bp (Utilities|Casting|CastToHuman_BP (.HitActor (Collision|BreakHitResult _outhit)))
          (:then
            (Variables|Default|SetAimedHuman (Utilities|ResolveSoftReference _ashuman_bp))
            (Widget|SetVisibility _crosshairgenderimage_2 "Visible")
            (if (== (Variables|/Game/Blueprints/Human_BP.Human_BP_C|GetGender _ashuman_bp) 0)
              (Appearance|SetBrushfromTexture _crosshairgenderimage_2 "/Game/Textures/female_icon.female_icon" false)
              (else
                (Appearance|SetBrushfromTexture _crosshairgenderimage_2 "/Game/Textures/male_icon.male_icon" false))))
          (:CastFailed
            (Variables|Default|SetAimedHuman 0)
            (Widget|SetVisibility _crosshairgenderimage_2 "Hidden")))
        (else
          (goto _label))))))

(event Input|ActionEvents|InputActionFire
  (params (Key :type Key%20Structure))
  (bind _aimedhuman (Variables|Default|GetAimedHuman))
  (bind _output (Utilities|ResolveSoftReference _aimedhuman))
  (:Pressed
    (Utilities|IsValid _output
      (:Is%20Valid
        (Default|ChangeGender _output)
        (Audio|PlaySoundatLocation "/Game/ChangeGender.ChangeGender" (Transformation|GetActorLocation _output) "0, 0, 0" 1.0 1.0 0.0 0 0 0)))))

(event Input|ActionEvents|InputActionQuit
  (params (Key :type Key%20Structure))
  (:Pressed
    (Game|QuitGame 0 "Quit")))

(event Input|AxisEvents|InputAxisTurn
  (params (AxisValue :type Float%20%28single-precision%29))
  (bind _asplayer_bp (Utilities|Casting|CastToPlayer_BP (Pawn|GetControlledPawn)))
  (Transformation|AddActorLocalRotation _asplayer_bp (Math|Rotator|MakeRotator 0.0 0.0 (* AxisValue (Variables|Default|GetTurnInputMultiplier))) false false))

(event Input|AxisEvents|InputAxisLoopUp
  (params (AxisValue :type Float%20%28single-precision%29))
  (bind _asplayer_bp (Utilities|Casting|CastToPlayer_BP (Pawn|GetControlledPawn)))
  (Transformation|AddLocalRotation (Variables|/Game/Blueprints/Player_BP.Player_BP_C|GetCamera _asplayer_bp) (Math|Rotator|MakeRotator 0.0 (* AxisValue (Variables|Default|GetTurnInputMultiplier)) 0.0) false false))

(event Input|AxisEvents|InputAxisMoveForward
  (params (AxisValue :type Float%20%28single-precision%29))
  (bind _ascharacter (Utilities|Casting|CastToCharacter (Pawn|GetControlledPawn)))
  (Physics|AddForce (Variables|/Script/Engine.Character|GetCapsuleComponent _ascharacter) (* (Math|Vector|GetForwardVector (Math|Rotator|MakeRotator (.Roll (Math|Rotator|BreakRotator (Transformation|GetActorRotation _ascharacter))) (.Pitch (Math|Rotator|BreakRotator (Transformation|GetActorRotation _ascharacter))) (.Yaw (Math|Rotator|BreakRotator (Transformation|GetActorRotation _ascharacter))))) (* AxisValue (Variables|Default|GetMoveInputMultiplier))) "None" false))

(event Input|AxisEvents|InputAxisMoveRight
  (params (AxisValue :type Float%20%28single-precision%29))
  (bind _ascharacter (Utilities|Casting|CastToCharacter (Pawn|GetControlledPawn)))
  (Physics|AddForce (Variables|/Script/Engine.Character|GetCapsuleComponent _ascharacter) (* (Math|Vector|GetRightVector (Math|Rotator|MakeRotator (.Roll (Math|Rotator|BreakRotator (Transformation|GetActorRotation _ascharacter))) (.Pitch (Math|Rotator|BreakRotator (Transformation|GetActorRotation _ascharacter))) (.Yaw (Math|Rotator|BreakRotator (Transformation|GetActorRotation _ascharacter))))) (* AxisValue (Variables|Default|GetMoveInputMultiplier))) "None" false))

(fn ConstructionScript)