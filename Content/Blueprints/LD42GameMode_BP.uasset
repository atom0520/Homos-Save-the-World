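; Game mode for a planet population game that ends when humans reach the maximum count or either gender drops to zero.
; BeginPlay creates the GUI and spawns both genders at random points around the planet.
; SpawnHuman reuses disabled pooled humans before spawning new AI, updating gender counts and GUI text.
; Tick checks end conditions to show game over with the cursor, while OnRestartGame reloads the map, leaving an in-place reset unused.
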(event EventBeginPlay
  (bind _humanspawnnumberpergender (Variables|Default|GetHumanSpawnNumberPerGender))
  (bind _returnvalue (UserInterface|CreateWidget "/Game/Blueprints/GUIWidget_BP.GUIWidget_BP_C"))
  (bind _output_get (Variables|Default|SetGUIWidget _returnvalue))
  (EventDispatchers|BindEventtoOnClicked (Variables|/Game/Blueprints/GUIWidget_BP.GUIWidget_BP_C|GetRestartButton _output_get) (EventDispatchers|CreateEvent :!event OnRestartGame))
  (UserInterface|Viewport|AddtoViewport _returnvalue 0)
  (bind _outactors (Actor|GetAllActorsOfClass "/Game/Blueprints/LocalDatabaseActor_BP.LocalDatabaseActor_BP_C"))
  (for _index (range 0 1)
    (CallFunction|UpdateNumberOfHumans _index _humanspawnnumberpergender)
    (for _index_2 (range 0 (- _humanspawnnumberpergender 1))
      (bind _returnvalue_2 (AI|SpawnAIFromClass "/Game/Blueprints/Human_BP.Human_BP_C" 0 (+ (Transformation|GetActorLocation (Variables|/Game/Blueprints/LocalDatabaseActor_BP.LocalDatabaseActor_BP_C|GetPlanet (Utilities|Array|Get(acopy) _outactors))) (Class|KismetMathLibrary|CreateVectorfromYawPitch (Math|Random|RandomFloatinRange -1.8e+02 1.8e+02) (Math|Random|RandomFloatinRange -1.8e+02 1.8e+02) (Variables|Default|GetHumanSpawnHeight))) "0, 0, 0" false))
      (bind _ashuman_bp (Utilities|Casting|CastToHuman_BP _returnvalue_2))
      (Default|Initialize _ashuman_bp _index false)
      (Utilities|Array|Add (Variables|Default|GetHumanPool) _ashuman_bp))))

(event EventTick
  (params (DeltaSeconds :type Float%20%28single-precision%29))
  (bind _returnvalue (Game|GetPlayerController 0))
  (bind _guiwidget (Variables|Default|GetGUIWidget))
  (if (not (Variables|Default|GetIsGameOver))
    (bind _returnvalue_2 (CallFunction|IsOutOfSpace))
    (if _returnvalue_2
      (Default|OnGameOver _guiwidget)
      (Input|SetInputModeGameandUI _returnvalue _guiwidget "DoNotLock" false :!label _label)
      (Variables|/Script/Engine.PlayerController|SetbShowMouseCursor _returnvalue true)
      (Variables|Default|SetIsGameOver true)
      (elif (== (Variables|Default|GetNumberOfWomen) 0)
        (Default|OnGameOver _guiwidget 1)
        (goto _label)
        (elif (== (Variables|Default|GetNumberOfMen) 0)
          (Default|OnGameOver _guiwidget 2)
          (goto _label))))))

(fn ConstructionScript)

(fn SpawnHuman
  (params (Location :type Vector) (Rotation :type Rotator) (Gender :type Integer) (Mature :type Boolean))
  (for _array_element (Variables|Default|GetHumanPool)
    (if (not (Variables|/Game/Blueprints/Human_BP.Human_BP_C|GetEnabled _array_element))
      (Default|Initialize _array_element Gender Mature)
      (Transformation|SetActorLocation _array_element Location false true)
      (Transformation|SetActorRotation _array_element Rotation true)
      (Default|SetEnabled _array_element true)
      (Utilities|Casting|CastToLD42GameMode_BP (Game|GetGameMode))
      (CallFunction|UpdateNumberOfHumans Gender 1)
      (return _array_element)))
  (bind _returnvalue (AI|SpawnAIFromClass "/Game/Blueprints/Human_BP.Human_BP_C" 0 Location Rotation false))
  (Utilities|IsValid _returnvalue
    (:Is%20Valid
      (bind _ashuman_bp (Utilities|Casting|CastToHuman_BP _returnvalue))
      (Default|Initialize _ashuman_bp Gender Mature)
      (Utilities|Array|Add (Variables|Default|GetHumanPool) _ashuman_bp)
      (Utilities|Casting|CastToLD42GameMode_BP (Game|GetGameMode))
      (CallFunction|UpdateNumberOfHumans Gender 1)
      (return _ashuman_bp))))

(fn IsOutOfSpace
  (return (<= (Variables|Default|GetMaxNumberOfHumans) (+ (Variables|Default|GetNumberOfMen) (Variables|Default|GetNumberOfWomen)))))

(fn UpdateNumberOfHumans
  (params (Gender :type Integer) (Delta :type Integer))
  (bind _guiwidget (Variables|Default|GetGUIWidget))
  (if (== Gender 0)
    (bind _output_get (Variables|Default|SetNumberOfWomen (+ (Variables|Default|GetNumberOfWomen) Delta)))
    (Variables|/Game/Blueprints/GUIWidget_BP.GUIWidget_BP_C|SetNumberOfWomenText _guiwidget (Utilities|String|ToString(Integer) _output_get))
    (else
      (bind _output_get_2 (Variables|Default|SetNumberOfMen (+ Delta (Variables|Default|GetNumberOfMen))))
      (Variables|/Game/Blueprints/GUIWidget_BP.GUIWidget_BP_C|SetNumberOfMenText _guiwidget (Utilities|String|ToString(Integer) _output_get_2))))
  (Variables|/Game/Blueprints/GUIWidget_BP.GUIWidget_BP_C|SetNumberOfHumansText _guiwidget (Utilities|String|Append (Utilities|String|ToString(Integer) (+ (Variables|Default|GetNumberOfMen) (Variables|Default|GetNumberOfWomen))) " / " (Utilities|String|ToString(Integer) (Variables|Default|GetMaxNumberOfHumans)))))

(fn OnRestartGame
  (Game|OpenLevel(byName) "GameMap")
  (Input|SetInputModeGameOnly (Game|GetPlayerController 0)))