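; Human character that lives on a spherical planet, with a gender and a child or adult state, driven by HumanAIController_BP.
; Each tick it aligns upright to the planet and applies a physics force toward its center unless a line trace finds ground within reach.
; Initialize and GrowUp set scale and ground distance; ChangeGender swaps material and updates game mode head counts.
; SetEnabled toggles ticking, collision, physics and visibility together.
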(event EventBeginPlay
  (CallFunction|Initialize (Variables|Default|GetGender) (Variables|Default|GetMature))
  (bind _outactors (Actor|GetAllActorsOfClass "/Game/Blueprints/LocalDatabaseActor_BP.LocalDatabaseActor_BP_C"))
  (Variables|Default|SetPlanet (Variables|/Game/Blueprints/LocalDatabaseActor_BP.LocalDatabaseActor_BP_C|GetPlanet (Utilities|Array|Get(acopy) _outactors)))
  (Collision|SetCollisionEnabled (Variables|Character|GetMesh) "NoCollision"))

(event Collision|EventActorBeginOverlap
  (params (OtherActor :type Actor%20Object%20Reference)))

(event EventTick
  (params (DeltaSeconds :type Float%20%28single-precision%29))
  (bind _returnvalue (Transformation|GetActorLocation))
  (bind _planet (Variables|Default|GetPlanet))
  (bind _planet_2 (Variables|Default|GetPlanet))
  (bind _returnvalue_2 (Transformation|GetActorLocation _planet))
  (bind _returnvalue_3 (- _returnvalue_2 _returnvalue))
  (bind _returnvalue_4 (Math|Vector|Normalize _returnvalue_3))
  (bind _returnvalue_5 (Math|Vector|NegateVector _returnvalue_4))
  (Utilities|IsValid _planet_2
    (:Is%20Valid
      (Transformation|SetActorRotation (Class|KismetMathLibrary|MakeRotfromYZ (Math|Vector|NegateVector (Math|Vector|Normalize (Math|Vector|CrossProduct (Math|Vector|GetForwardVector (Transformation|GetActorRotation)) _returnvalue_5))) _returnvalue_5))
      (bind _outhit (Collision|LineTraceByChannel (Transformation|GetActorLocation) (Transformation|GetActorLocation _planet_2) "TraceTypeQuery3" false 0 "None" true "(R=1.000000,G=0.000000,B=0.000000,A=1.000000)" "(R=0.000000,G=1.000000,B=0.000000,A=1.000000)" DeltaSeconds))
      (if (not (<= (.Distance (Collision|BreakHitResult _outhit)) (Variables|Default|GetDistanceToGround)))
        (Physics|AddForce (Variables|Collision|GetCapsuleComponent) (* _returnvalue_4 (Variables|Default|GetGravityMultiplier)) "None" false)))))

(fn ConstructionScript)

(fn SetEnabled
  (params (Enabled :type Boolean))
  (Variables|Default|SetEnabled Enabled)
  (Actor|Tick|SetActorTickEnabled Enabled)
  (Actor|Tick|SetActorTickEnabled (Pawn|GetController) Enabled)
  (Collision|SetActorEnableCollision Enabled)
  (Physics|SetSimulatePhysics (Variables|Collision|GetCapsuleComponent) Enabled)
  (Rendering|SetActorHiddenInGame (not Enabled)))

(fn GrowUp
  (Variables|Default|SetMature true)
  (Transformation|SetActorScale3D "1.000000,1.000000,1.000000")
  (Variables|Default|SetDistanceToGround 9e+01))

(fn Initialize
  (params (Gender :type Integer) (Mature :type Boolean))
  (bind _mesh (Variables|Character|GetMesh))
  (Variables|Default|SetGender Gender)
  (Variables|Default|SetMature Mature)
  (Utilities|FlowControl|Sequence
    (:then_0
      (if (Variables|Default|GetMature)
        (Transformation|SetActorScale3D "1.000000,1.000000,1.000000")
        (Variables|Default|SetDistanceToGround 9e+01)
        (else
          (Transformation|SetActorScale3D "0.600000,0.600000,0.600000")
          (Variables|Default|SetDistanceToGround 54.0))))
    (:then_1
      (if (Math|Conversions|ToBoolean(Integer) (Variables|Default|GetGender))
        (Rendering|Material|SetMaterial _mesh 0 "/Game/Materials/HumanMale.HumanMale")
        (else
          (Rendering|Material|SetMaterial _mesh 0 "/Game/Materials/HumanFemale.HumanFemale"))))
    (:then_2
      (bind _ashuman_aicontroller_bp (Utilities|Casting|CastToHumanAIController_BP (Pawn|GetController)))
      (Default|Initialize _ashuman_aicontroller_bp))))

(fn ChangeGender
  (bind _returnvalue (Game|GetGameMode))
  (bind _mesh (Variables|Character|GetMesh))
  (if (== (Variables|Default|GetGender) 0)
    (Variables|Default|SetGender 1)
    (Rendering|Material|SetMaterial _mesh 0 "/Game/Materials/HumanMale.HumanMale")
    (bind _asld42game_mode_bp (Utilities|Casting|CastToLD42GameMode_BP _returnvalue))
    (Default|UpdateNumberOfHumans _asld42game_mode_bp 1 1)
    (Default|UpdateNumberOfHumans _asld42game_mode_bp 0 -1)
    (else
      (Variables|Default|SetGender 0)
      (Rendering|Material|SetMaterial _mesh 0 "/Game/Materials/HumanFemale.HumanFemale")
      (bind _asld42game_mode_bp_2 (Utilities|Casting|CastToLD42GameMode_BP _returnvalue))
      (Default|UpdateNumberOfHumans _asld42game_mode_bp_2 1 -1)
      (Default|UpdateNumberOfHumans _asld42game_mode_bp_2 0 1))))