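; Human actor (old version) that lives on a spherical planet, with a gender and a child or adult state.
; Tick aligns it to the planet's surface and applies custom gravity as capsule force until a downward trace reaches ground distance.
; Initialize sets scale, ground distance and gendered material, then initializes its AI controller.
; GrowUp matures it, ChangeGender updates GameMode headcounts, and SetEnabled toggles tick, collision, physics and visibility.
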(event EventBeginPlay
  (CallFunction|Initialize (Variables|Default|GetGender) (Variables|Default|GetMature))
  (bind _outactors (Actor|GetAllActorsOfClass "/Game/Blueprints/BP_LocalDatabaseActor.BP_LocalDatabaseActor_C"))
  (Variables|Default|SetPlanet (Variables|/Game/Blueprints/BP_LocalDatabaseActor.BP_LocalDatabaseActor_C|GetPlanet (Utilities|Array|Get(acopy) _outactors)))
  (Collision|SetCollisionEnabled (Variables|Default|GetMesh) "NoCollision"))

(event Collision|EventActorBeginOverlap
  (params (OtherActor :type Actor%20Object%20Reference)))

(event EventTick
  (params (DeltaSeconds :type Float%20%28single-precision%29))
  (bind _returnvalue (Transformation|GetActorRotation))
  (bind _returnvalue_2 (Transformation|GetActorLocation))
  (bind _planet (Variables|Default|GetPlanet))
  (bind _planet_2 (Variables|Default|GetPlanet))
  (bind _returnvalue_3 (Transformation|GetActorLocation _planet))
  (bind _returnvalue_4 (Math|Vector|GetForwardVector _returnvalue))
  (bind _returnvalue_5 (- _returnvalue_3 _returnvalue_2))
  (bind _returnvalue_6 (Math|Vector|Normalize _returnvalue_5))
  (bind _returnvalue_7 (Math|Vector|NegateVector _returnvalue_6))
  (Utilities|IsValid _planet_2
    (:Is%20Valid
      (Transformation|SetActorRotation (Math|Rotator|MakeRotfromXZ (- _returnvalue_4 (Math|Vector|ProjectVectorontoVector _returnvalue_4 _returnvalue_7)) _returnvalue_7))
      (bind _outhit (Collision|LineTraceByChannel (Transformation|GetActorLocation) (Transformation|GetActorLocation _planet_2) "TraceTypeQuery3" false 0 "None" true "(R=1.000000,G=0.000000,B=0.000000,A=1.000000)" "(R=0.000000,G=1.000000,B=0.000000,A=1.000000)" DeltaSeconds))
      (if (not (<= (.Distance (Collision|BreakHitResult _outhit)) (Variables|Default|GetDistanceToGround)))
        (Physics|AddForce (Variables|Default|GetCapsuleComponent) (* _returnvalue_6 (Variables|Default|GetGravityMultiplier)) "None" false)))))

(fn ConstructionScript)

(fn SetEnabled
  (params (Enabled :type Boolean))
  (Variables|Default|SetEnabled Enabled)
  (Actor|Tick|SetActorTickEnabled Enabled)
  (Actor|Tick|SetActorTickEnabled (Pawn|GetController) Enabled)
  (Collision|SetActorEnableCollision Enabled)
  (Physics|SetSimulatePhysics (Variables|Default|GetCapsuleComponent) Enabled)
  (Rendering|SetActorHiddenInGame (not Enabled)))

(fn GrowUp
  (Variables|Default|SetMature true)
  (Transformation|SetActorScale3D "1.000000,1.000000,1.000000")
  (Variables|Default|SetDistanceToGround 9e+01))

(fn Initialize
  (params (Gender :type Integer) (Mature :type Boolean))
  (bind _mesh (Variables|Default|GetMesh))
  (Variables|Default|SetGender Gender)
  (Variables|Default|SetMature Mature)
  (Utilities|FlowControl|Sequence
    (:then_0
      (if (Variables|Default|GetMature)
        (Transformation|SetActorScale3D "1.000000,1.000000,1.000000")
        (Variables|Default|SetDistanceToGround 9e+01)
        (else
          (Transformation|SetActorScale3D "0.600000,0.600000,0.600000")
          (Variables|Default|SetDistanceToGround 54.0))))
    (:then_1
      (if (Math|Conversions|ToBoolean(Integer) (Variables|Default|GetGender))
        (Rendering|Material|SetMaterial _mesh 0 "/Game/Materials/M_HumanMan.M_HumanMan")
        (else
          (Rendering|Material|SetMaterial _mesh 0 "/Game/Materials/M_HumanWoman.M_HumanWoman"))))
    (:then_2
      (bind _asbp_human_aicontroller_old (Utilities|Casting|CastToBP_HumanAIController_Old (Pawn|GetController)))
      (Default|Initialize _asbp_human_aicontroller_old))))

(fn ChangeGender
  (bind _returnvalue (Game|GetGameMode))
  (bind _mesh (Variables|Default|GetMesh))
  (if (== (Variables|Default|GetGender) 0)
    (Variables|Default|SetGender 1)
    (Rendering|Material|SetMaterial _mesh 0 "/Game/Materials/M_HumanMan.M_HumanMan")
    (bind _asbp_ld42game_mode_old (Utilities|Casting|CastToBP_LD42GameMode_Old _returnvalue))
    (Default|UpdateNumberOfHumans _asbp_ld42game_mode_old 1 1)
    (Default|UpdateNumberOfHumans _asbp_ld42game_mode_old 0 -1)
    (else
      (Variables|Default|SetGender 0)
      (Rendering|Material|SetMaterial _mesh 0 "/Game/Materials/M_HumanWoman.M_HumanWoman")
      (bind _asbp_ld42game_mode_old_2 (Utilities|Casting|CastToBP_LD42GameMode_Old _returnvalue))
      (Default|UpdateNumberOfHumans _asbp_ld42game_mode_old_2 1 -1)
      (Default|UpdateNumberOfHumans _asbp_ld42game_mode_old_2 0 1))))