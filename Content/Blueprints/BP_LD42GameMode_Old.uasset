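; Game mode for a planet population game that tracks men and women and ends on overcrowding or either gender dying out.
; BeginPlay creates the GUI and spawns immature AI humans at random points around the planet.
; SpawnHuman reuses disabled pawns from HumanPool0 before spawning new ones, updating counts and GUI text.
; Tick checks game-over conditions; OnRestartGame reloads GameMap, leaving an in-place pool reset unreachable.
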(event EventBeginPlay
  (bind _humanspawnnumberpergender_0 (Variables|Default|GetHumanSpawnNumberPerGender_0))
  (Development|PrintString "LD42GameMode_BP.BeginPlay" true true "(R=1.000000,G=1.000000,B=0.000000,A=1.000000)")
  (bind _returnvalue (UserInterface|CreateWidget "/Game/Blueprints/BP_GUIWidget.BP_GUIWidget_C"))
  (bind _output_get (Variables|Default|SetGUIWidget_0 _returnvalue))
  (EventDispatchers|BindEventtoOnClicked (Variables|/Game/Blueprints/BP_GUIWidget.BP_GUIWidget_C|GetRestartButton _output_get) (EventDispatchers|CreateEvent :!event OnRestartGame))
  (UserInterface|Viewport|AddtoViewport _returnvalue 0)
  (bind _outactors (Actor|GetAllActorsOfClass "/Game/Blueprints/BP_LocalDatabaseActor.BP_LocalDatabaseActor_C"))
  (for _index (range 0 1)
    (CallFunction|UpdateNumberOfHumans _index _humanspawnnumberpergender_0)
    (for _index_2 (range 0 (- _humanspawnnumberpergender_0 1))
      (bind _returnvalue_2 (AI|SpawnAIFromClass "/Game/Blueprints/BP_Human_Old.BP_Human_Old_C" 0 (+ (Transformation|GetActorLocation (Variables|/Game/Blueprints/BP_LocalDatabaseActor.BP_LocalDatabaseActor_C|GetPlanet (Utilities|Array|Get(acopy) _outactors))) (Class|KismetMathLibrary|CreateVectorfromYawPitch (Math|Random|RandomFloatinRange -1.8e+02 1.8e+02) (Math|Random|RandomFloatinRange -1.8e+02 1.8e+02) (Variables|Default|GetHumanSpawnHeight_0))) "0, 0, 0" false))
      (bind _asbp_human_old (Utilities|Casting|CastToBP_Human_Old _returnvalue_2))
      (Default|Initialize _asbp_human_old _index false)
      (Utilities|Array|Add (Variables|Default|GetHumanPool_0) _asbp_human_old))))

(event EventTick
  (params (DeltaSeconds :type Float%20%28single-precision%29))
  (bind _returnvalue (Game|GetPlayerController 0))
  (bind _guiwidget_0 (Variables|Default|GetGUIWidget_0))
  (if (not (Variables|Default|GetIsGameOver))
    (bind _returnvalue_2 (CallFunction|IsOutOfSpace))
    (if _returnvalue_2
      (Default|OnGameOver _guiwidget_0)
      (Input|SetInputModeGameandUI _returnvalue _guiwidget_0 "DoNotLock" false :!label _label)
      (Variables|/Script/Engine.PlayerController|SetbShowMouseCursor _returnvalue true)
      (Variables|Default|SetIsGameOver true)
      (elif (== (Variables|Default|GetNumberOfWomen) 0)
        (Default|OnGameOver _guiwidget_0 1)
        (goto _label)
        (elif (== (Variables|Default|GetNumberOfMen) 0)
          (Default|OnGameOver _guiwidget_0 2)
          (goto _label))))))

(fn ConstructionScript)

(fn SpawnHuman
  (params (Location :type Vector) (Rotation :type Rotator) (Gender :type Integer) (Mature :type Boolean))
  (for _array_element (Variables|Default|GetHumanPool_0)
    (if (not (Variables|/Game/Blueprints/BP_Human_Old.BP_Human_Old_C|GetEnabled _array_element))
      (Default|Initialize _array_element Gender Mature)
      (Transformation|SetActorLocation _array_element Location false true)
      (Transformation|SetActorRotation _array_element Rotation true)
      (Default|SetEnabled _array_element true)
      (Utilities|Casting|CastToBP_LD42GameMode_Old (Game|GetGameMode))
      (CallFunction|UpdateNumberOfHumans Gender 1)
      (return _array_element)))
  (bind _returnvalue (AI|SpawnAIFromClass "/Game/Blueprints/BP_Human_Old.BP_Human_Old_C" 0 Location Rotation false))
  (Utilities|IsValid _returnvalue
    (:Is%20Valid
      (bind _asbp_human_old (Utilities|Casting|CastToBP_Human_Old _returnvalue))
      (Default|Initialize _asbp_human_old Gender Mature)
      (Utilities|Array|Add (Variables|Default|GetHumanPool_0) _asbp_human_old)
      (Utilities|Casting|CastToBP_LD42GameMode_Old (Game|GetGameMode))
      (CallFunction|UpdateNumberOfHumans Gender 1)
      (return _asbp_human_old))))

(fn IsOutOfSpace
  (return (<= (Variables|Default|GetMaxNumberOfHumans) (+ (Variables|Default|GetNumberOfMen) (Variables|Default|GetNumberOfWomen)))))

(fn UpdateNumberOfHumans
  (params (Gender :type Integer) (Delta :type Integer))
  (bind _guiwidget_0 (Variables|Default|GetGUIWidget_0))
  (if (== Gender 0)
    (bind _output_get (Variables|Default|SetNumberOfWomen (+ (Variables|Default|GetNumberOfWomen) Delta)))
    (Variables|/Game/Blueprints/BP_GUIWidget.BP_GUIWidget_C|SetNumberOfWomenText _guiwidget_0 (Utilities|String|ToString(Integer) _output_get))
    (else
      (bind _output_get_2 (Variables|Default|SetNumberOfMen (+ Delta (Variables|Default|GetNumberOfMen))))
      (Variables|/Game/Blueprints/BP_GUIWidget.BP_GUIWidget_C|SetNumberOfMenText _guiwidget_0 (Utilities|String|ToString(Integer) _output_get_2))))
  (Variables|/Game/Blueprints/BP_GUIWidget.BP_GUIWidget_C|SetNumberOfHumansText _guiwidget_0 (Utilities|String|Append (Utilities|String|ToString(Integer) (+ (Variables|Default|GetNumberOfMen) (Variables|Default|GetNumberOfWomen))) " / " (Utilities|String|ToString(Integer) (Variables|Default|GetMaxNumberOfHumans)))))

(fn OnRestartGame
  (Game|OpenLevel(byName) "GameMap")
  (Input|SetInputModeGameOnly (Game|GetPlayerController 0)))